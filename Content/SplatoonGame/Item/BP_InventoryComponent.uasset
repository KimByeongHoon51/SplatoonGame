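; Inventory component for the Splatoon-style game, holding an array of item slots that is filled with five "Empty" entries on BeginPlay.
; Item data comes from DT_Item by row name, with the "Empty" row serving as the sentinel for a free slot.
; AddItem writes to the first free slot without checking the full flag, RemoveItem resets a slot to "Empty", and SwapItem exchanges two slots.
; PrintAllSlot prints slot contents for debugging.
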(event `self.ReceiveBeginPlay`
  (`self.CreateInvenSlots` 5))

(fn `AddItem`
  (params (RowName :type Name))
  (if (!= RowName "Empty")
    (bind _returnvalue (`|GetDataTableRow` "/Game/SplatoonGame/Item/DT_Item.DT_Item" RowName)
      (:`then`
        (bind _index (`self.FindEmptySlot`))
        (`KismetArrayLibrary.Array_Set` (`self.Slots`) _index (make `/Game/SplatoonGame/Item/ST_ItemSlot` 1 _returnvalue))))))

(fn `CreateInvenSlots`
  (params (Count :type Integer))
  (for _ (range Count)
    (bind _returnvalue (`|GetDataTableRow` "/Game/SplatoonGame/Item/DT_Item.DT_Item" "Empty")
      (:`then`
        (`KismetArrayLibrary.Array_Add` (`self.Slots`) (make `/Game/SplatoonGame/Item/ST_ItemSlot` Count _returnvalue))))))

(fn `FindEmptySlot`
  (returns (Index :type Integer) (IsFull :type Boolean))
  (for (_ _array_index) (`self.Slots`)
    (if (`self.IsEmptySlot` _array_index)
      (return _array_index false)))
  (return -1 true))

(fn `IsEmptySlot`
  (params (Index :type Integer))
  (returns (IsEmpty :type Boolean))
  (return (`KismetStringLibrary.EqualEqual_StrStr` (break `/Game/SplatoonGame/Item/ST_Item` (`.ItemData_3_94018485477A58AB8D84C7ADCA0DDDDA` (break `/Game/SplatoonGame/Item/ST_ItemSlot` (`|GetArrayItem` (`self.Slots`) Index)))) "Empty")))

(fn `PrintAllSlot`
  (for (_array_element _array_index) (`self.Slots`)
    (`KismetSystemLibrary.PrintString` (`KismetStringLibrary.Concat_StrStr` "Index:  " (`KismetStringLibrary.Conv_IntToString` _array_index) "Name: " (break `/Game/SplatoonGame/Item/ST_Item` (`.ItemData_3_94018485477A58AB8D84C7ADCA0DDDDA` (break `/Game/SplatoonGame/Item/ST_ItemSlot` _array_element)))) true true (struct :`G` 0.66 :`B` 1.0 :`A` 1.0) 30.0)))

(fn `RemoveItem`
  (params (Index :type Integer))
  (`self.SetEmptySlot` Index))

(fn `SetEmptySlot`
  (params (Index :type Integer))
  (bind _returnvalue (`|GetDataTableRow` "/Game/SplatoonGame/Item/DT_Item.DT_Item" "Empty")
    (:`then`
      (setmembers `/Game/SplatoonGame/Item/ST_ItemSlot` :`StructRef` (`|GetArrayItem` (`self.Slots`) Index) :`ItemData` _returnvalue))))

(fn `SwapItem`
  (params (FromIndex :type Integer) (ToIndex :type Integer))
  (`KismetArrayLibrary.Array_Swap` (`self.Slots`) FromIndex ToIndex))